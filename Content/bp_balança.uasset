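; An overlap-triggered actor, named bp_balança (scale), that lights up and shows a text label while another actor overlaps it.
; BeginPlay applies the Cor color variable to the point light, sets the text render to the Texto variable and hides it.
; Overlap begin raises the light intensity and reveals the text; overlap end zeroes the light and hides the text, without tracking which actor or how many overlap.
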(event `self.ReceiveActorBeginOverlap`
  (params (OtherActor :type "Actor Object Reference"))
  (`LightComponent.SetIntensity` (`self.PointLight`) 5000.0)
  (`SceneComponent.SetVisibility` (`self.TextRender`) true false))

(event `self.ReceiveActorEndOverlap`
  (params (OtherActor :type "Actor Object Reference"))
  (`LightComponent.SetIntensity` (`self.PointLight`) 0.0)
  (`SceneComponent.SetVisibility` (`self.TextRender`) false false))

(event `self.ReceiveBeginPlay`
  (`LightComponent.SetLightColor` (`self.PointLight`) (`self.cor`) true)
  (`TextRenderComponent.K2_SetText` (`self.TextRender`) (`self.texto`))
  (`SceneComponent.SetVisibility` (`self.TextRender`) false false))

(fn `UserConstructionScript`)